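; Master Poggermon creature Blueprint, whose Follower movement type trails the QuikishRef actor.
; BeginPlay sets the follower walk speed and starts FollowerServer, a self-calling event that re-issues AIMoveTo toward QuikishRef's FollowerSphere after half-second delays.
; When too far away, it teleports to a world-X offset from the target and immediately re-evaluates.
; Both near-distance branches perform the same move, and debug prints remain.
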(event `self.ReceiveActorBeginOverlap`
  (params (OtherActor :type "Actor Object Reference")))

(event `self.ReceiveBeginPlay`
  (bind _follower_speed (`self.Follower Speed`))
  (switch `/Game/CreatureInfo/EPoggermonMovementType` (`self.Movement Type`)
    (:`NewEnumerator1`
      (`KismetSystemLibrary.PrintString` (`KismetStringLibrary.Conv_DoubleToString` _follower_speed))
      (set `CharacterMovementComponent.MaxWalkSpeed` _follower_speed (`self.CharacterMovement`))
      (`self.Follower Server`))))

(event `Follower Server`
  (bind (_returnvalue_x _returnvalue_y _returnvalue_z) (`KismetMathLibrary.BreakVector` (`self.K2_GetActorLocation` (`self.Quikish Ref`))))
  (bind _returnvalue (`SceneComponent.K2_GetComponentLocation` (`/Game/VRTemplate/Blueprints/VRPawn.FollowerSphere` (`self.Quikish Ref`))))
  (if (>= (`self.GetDistanceTo` (`self.Quikish Ref`)) 1500.0)
    (`self.K2_SetActorLocation` (`KismetMathLibrary.MakeVector` (- _returnvalue_x 100.0) _returnvalue_y _returnvalue_z) false true)
    (`self.Follower Server`)
    (else
      (if (>= (`self.GetDistanceTo` (`self.Quikish Ref`)) 200.0)
        (`|AIMoveTo` self _returnvalue null
          (:`then`
            _))
        (else
          (`|AIMoveTo` self _returnvalue null
            (:`then`
              _))))
      (`KismetSystemLibrary.Delay` 0.5)
      (`KismetSystemLibrary.PrintString` (`KismetStringLibrary.Conv_VectorToString` _returnvalue))
      (`self.Follower Server`))))

(fn `UserConstructionScript`)