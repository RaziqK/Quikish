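; Wild Poggermon encounter zone that starts a single-opponent battle while the VRPawn moves inside its box.
; A looping timer rolls each second, with odds rising after each failure, and pauses on success.
; SetEncounter picks a weighted species, then rolls shininess, gender, route-based level, IVs, stats and up to four level-up moves before calling SPBattleStart on the pawn.
; Stats always use the Timid nature; FindNature is never called.
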(event OnComponentBeginOverlap(Box)
  (params (OverlappedComponent :type Primitive%20Component%20Object%20Reference) (OtherActor :type Actor%20Object%20Reference) (OtherComp :type Primitive%20Component%20Object%20Reference) (OtherBodyIndex :type Integer) (bFromSweep :type Boolean) (SweepResult :type Hit%20Result%20Structure%20%28by%20ref%29))
  (bind _asvrpawn (Utilities|Casting|CastToVRPawn OtherActor))
  (Utilities|IsValid (Game|GetPlayerController 0)
    (:Is%20Valid
      (Development|PrintString "valid")
      (bind _output_get (Variables|Default|SetQuikish%20Ref _asvrpawn))
      (Variables|/Game/VRTemplate/Blueprints/VRPawn.VRPawn_C|SetEncounterBoxRef _output_get self)
      (bind _returnvalue (Utilities|Time|SetTimerbyEvent (delegate Custom|RollEncounter) 1.0 true))
      (Variables|Default|SetSpawn%20Timer _returnvalue))
    (:Is%20Not%20Valid
      (Development|PrintString "Invalid"))))

(event OnComponentEndOverlap(Box)
  (params (OverlappedComponent :type Primitive%20Component%20Object%20Reference) (OtherActor :type Actor%20Object%20Reference) (OtherComp :type Primitive%20Component%20Object%20Reference) (OtherBodyIndex :type Integer))
  (Utilities|Casting|CastToVRPawn OtherActor)
  (Utilities|Time|ClearandInvalidateTimerbyHandle (Variables|Default|GetSpawn%20Timer)))

(event Custom|RollEncounter
  (if (> (Math|Vector|VectorLengthXY (Variables|/Script/Engine.MovementComponent|GetVelocity (Variables|/Script/Engine.Character|GetCharacterMovement (Variables|Default|GetQuikish%20Ref)))) 0.1)
    (if (Math|Random|RandomBoolwithWeight (+ (Math|Float|MakeLiteralFloat 0.1) (* (Variables|Default|GetTimes%20Roll%20Failed) 0.05)))
      (Variables|Default|SetTimes%20Roll%20Failed 0)
      (Utilities|Time|PauseTimerbyHandle (Variables|Default|GetSpawn%20Timer))
      (CallFunction|SetEncounter)
      (else
        (Math|Integer|IncrementInt (Variables|Default|GetTimes%20Roll%20Failed))))))

(event Custom|Set%20Encounter
  (Utilities|Array|Clear (Variables|Default|GetEnemyTeam))
  (if (== (Math|Random|RandomIntegerinRange 1 4096) 1)
    (Variables|PoggermonInfo|SetIsShiny true)
    (else
      (Variables|PoggermonInfo|SetIsShiny false)))
  (if (>= (Math|Random|RandomInteger 100) 51)
    (Variables|PoggermonInfo|SetGender "NewEnumerator1")
    (else
      (Variables|PoggermonInfo|SetGender "NewEnumerator2")))
  (bind _poggermon_name (CallFunction|ChooseEncounter))
  (bind _returnvalue (Utilities|GetDataTableRow "/Game/CreatureInfo/PoggermonBasicInfoDT.PoggermonBasicInfoDT" _poggermon_name)
    (:then
      (CallFunction|SetEncounterInfo _returnvalue)
      (CallFunction|RollIV)
      (CallFunction|RollFinalStats _poggermon_name)
      (CallFunction|RollMoveSlots)
      (Utilities|Array|Add (Variables|Default|GetEnemyTeam) (Variables|Default|GetEncounterPoggermon))
      (bind _asvrpawn (Utilities|Casting|CastToVRPawn (Game|GetPlayerCharacter 0))
        (:then
          (Default|SPBattleStart _asvrpawn (Variables|Default|GetEnemyTeam) (Variables|Default|GetEnemy%20Inventory)))
        (:CastFailed
          (Development|PrintString "Failed Cast at Encounter BP"))))))

(fn ConstructionScript)

(fn ChooseEncounter
  (bind _possiblepoggermon (Variables|Default|GetPossiblePoggermon))
  (bind _poggermonname (Utilities|Struct|BreakFPossibleEncounters _possiblepoggermon))
  (LocalVariables|SetSum%20of%20Array 0.0)
  (bind _values (Utilities|Map|Values (Utilities|Struct|BreakFPossibleEncounters (Variables|Default|GetPossiblePoggermon))))
  (for _array_element _values
    (LocalVariables|SetSum%20of%20Array (+ (LocalVariables|GetSum%20of%20Array) _array_element)))
  (LocalVariables|SetRoll (Math|Random|RandomFloatinRange 0.0 (LocalVariables|GetSum%20of%20Array)))
  (bind _keys (Utilities|Map|Keys _poggermonname))
  (bind _array_element_2 (Utilities|Array|ForEachLoopwithBreak _keys :!label _label)
    (:LoopBody
      (if (>= (.Value (Utilities|Map|Find _poggermonname _array_element_2)) (LocalVariables|GetRoll))
        (LocalVariables|SetChosenEncounter _array_element_2)
        (goto _label Break)
        (else
          (LocalVariables|SetRoll (- (LocalVariables|GetRoll) (.Value (Utilities|Map|Find _poggermonname _array_element_2)))))))
    (:Completed
      (return (LocalVariables|GetChosenEncounter)))))

(fn SetEncounterInfo
  (params (Poggermon%20Base%20Info :type F%20Poggermon%20Basic%20Information%20Structure))
  (bind _poggermonname (Utilities|Struct|BreakFPoggermonBasicInformation Poggermon%20Base%20Info))
  (bind _returnvalue (Utilities|GetDataTableRow (Variables|Default|GetRoute%20Info) _poggermonname)
    (:then
      (bind _structout (Utilities|Struct|SetmembersinFPoggermonPartyInfo (Variables|Default|GetEncounterPoggermon) _poggermonname (Utilities|String|ToString(Name) _poggermonname) (Math|Random|RandomIntegerinRange (.MinimumLevel (Utilities|Struct|BreakFEncounterStruct _returnvalue)) (.MaximumLevel (Utilities|Struct|BreakFEncounterStruct _returnvalue))) (Variables|PoggermonInfo|GetGender) (Variables|PoggermonInfo|GetIsShiny)))
      (Variables|Default|SetEncounterPoggermon _structout)
      (return))))

(fn RollIV
  (bind _structout (Utilities|Struct|SetmembersinFPoggermonPartyInfo (Variables|Default|GetEncounterPoggermon) (Utilities|Struct|MakeFPoggermonIV (Math|Random|RandomIntegerinRange 0 31) (Math|Random|RandomIntegerinRange 0 31) (Math|Random|RandomIntegerinRange 0 31) (Math|Random|RandomIntegerinRange 0 31) (Math|Random|RandomIntegerinRange 0 31) (Math|Random|RandomIntegerinRange 0 31))))
  (Variables|Default|SetEncounterPoggermon _structout)
  (return))

(fn RollFinalStats
  (params (Poggermon%20Name :type Name))
  (bind _returnvalue (Utilities|GetDataTableRow "/Game/CreatureInfo/PoggermonBasicInfoDT.PoggermonBasicInfoDT" Poggermon%20Name)
    (:then
      (bind _returnvalue_2 (Utilities|GetDataTableRow "/Game/CreatureInfo/NaturesDT.NaturesDT" "Timid")
        (:then
          (bind _structout (Utilities|Struct|SetmembersinFPoggermonPartyInfo (Variables|Default|GetEncounterPoggermon) (/ (* (* (* (.CurrentLevel (Utilities|Struct|BreakFPoggermonPartyInfo (Variables|Default|GetEncounterPoggermon))) 4) (.CurrentLevel (Utilities|Struct|BreakFPoggermonPartyInfo (Variables|Default|GetEncounterPoggermon)))) (.CurrentLevel (Utilities|Struct|BreakFPoggermonPartyInfo (Variables|Default|GetEncounterPoggermon)))) 5) (.BaseStatInformation (Utilities|Struct|BreakFPoggermonBasicInformation _returnvalue)) (Utilities|Struct|MakeFPoggermonFinalStats (Math|Conversions|ToFloat(Integer) (Math|Float|Round (|((((((HPBS*2)+HP)*CL)/100)+CL)+10) (.HP (Utilities|Struct|BreakFPoggermonBaseStats (.BaseStatInformation (Utilities|Struct|BreakFPoggermonBasicInformation _returnvalue)))) (.HP (Utilities|Struct|BreakFPoggermonIV (.PoggerIV (Utilities|Struct|BreakFPoggermonPartyInfo (Variables|Default|GetEncounterPoggermon))))) (Utilities|Struct|BreakFPoggermonPartyInfo (Variables|Default|GetEncounterPoggermon))))) (Math|Conversions|ToFloat(Integer) (Math|Float|Round (|((((((HPBS*2)+HP)*CL)/100)+CL)+10) (.HP (Utilities|Struct|BreakFPoggermonBaseStats (.BaseStatInformation (Utilities|Struct|BreakFPoggermonBasicInformation _returnvalue)))) (.HP (Utilities|Struct|BreakFPoggermonIV (.PoggerIV (Utilities|Struct|BreakFPoggermonPartyInfo (Variables|Default|GetEncounterPoggermon))))) (Utilities|Struct|BreakFPoggermonPartyInfo (Variables|Default|GetEncounterPoggermon))))) (Math|Conversions|ToFloat(Integer) (Math|Float|Round (|(((((((StatBS*2)+IV)*CL)/100)+CL)+5)*MP) (.Attack (Utilities|Struct|BreakFPoggermonBaseStats (.BaseStatInformation (Utilities|Struct|BreakFPoggermonBasicInformation _returnvalue)))) (.Attack (Utilities|Struct|BreakFPoggermonIV (.PoggerIV (Utilities|Struct|BreakFPoggermonPartyInfo (Variables|Default|GetEncounterPoggermon))))) (Utilities|Struct|BreakFPoggermonPartyInfo (Variables|Default|GetEncounterPoggermon)) (.Value (Utilities|Map|Find (.Stats (Utilities|Struct|BreakFNatures _returnvalue_2)) "Attack"))))) (Math|Conversions|ToFloat(Integer) (Math|Float|Round (|(((((((StatBS*2)+IV)*CL)/100)+CL)+5)*MP) (.Attack (Utilities|Struct|BreakFPoggermonBaseStats (.BaseStatInformation (Utilities|Struct|BreakFPoggermonBasicInformation _returnvalue)))) (.Attack (Utilities|Struct|BreakFPoggermonIV (.PoggerIV (Utilities|Struct|BreakFPoggermonPartyInfo (Variables|Default|GetEncounterPoggermon))))) (Utilities|Struct|BreakFPoggermonPartyInfo (Variables|Default|GetEncounterPoggermon)) (.Value (Utilities|Map|Find (.Stats (Utilities|Struct|BreakFNatures _returnvalue_2)) "Attack"))))) (Math|Conversions|ToFloat(Integer) (Math|Float|Round (|(((((((StatBS*2)+IV)*CL)/100)+CL)+5)*MP) (.Defense (Utilities|Struct|BreakFPoggermonBaseStats (.BaseStatInformation (Utilities|Struct|BreakFPoggermonBasicInformation _returnvalue)))) (.Defense (Utilities|Struct|BreakFPoggermonIV (.PoggerIV (Utilities|Struct|BreakFPoggermonPartyInfo (Variables|Default|GetEncounterPoggermon))))) (Utilities|Struct|BreakFPoggermonPartyInfo (Variables|Default|GetEncounterPoggermon)) (.Value (Utilities|Map|Find (.Stats (Utilities|Struct|BreakFNatures _returnvalue_2)) "Defense"))))) (Math|Conversions|ToFloat(Integer) (Math|Float|Round (|(((((((StatBS*2)+IV)*CL)/100)+CL)+5)*MP) (.Defense (Utilities|Struct|BreakFPoggermonBaseStats (.BaseStatInformation (Utilities|Struct|BreakFPoggermonBasicInformation _returnvalue)))) (.Defense (Utilities|Struct|BreakFPoggermonIV (.PoggerIV (Utilities|Struct|BreakFPoggermonPartyInfo (Variables|Default|GetEncounterPoggermon))))) (Utilities|Struct|BreakFPoggermonPartyInfo (Variables|Default|GetEncounterPoggermon)) (.Value (Utilities|Map|Find (.Stats (Utilities|Struct|BreakFNatures _returnvalue_2)) "Defense"))))) (Math|Conversions|ToFloat(Integer) (Math|Float|Round (|(((((((StatBS*2)+IV)*CL)/100)+CL)+5)*MP) (.SPAttack (Utilities|Struct|BreakFPoggermonBaseStats (.BaseStatInformation (Utilities|Struct|BreakFPoggermonBasicInformation _returnvalue)))) (.SPAttack (Utilities|Struct|BreakFPoggermonIV (.PoggerIV (Utilities|Struct|BreakFPoggermonPartyInfo (Variables|Default|GetEncounterPoggermon))))) (Utilities|Struct|BreakFPoggermonPartyInfo (Variables|Default|GetEncounterPoggermon)) (.Value (Utilities|Map|Find (.Stats (Utilities|Struct|BreakFNatures _returnvalue_2)) "SP Attack"))))) (Math|Conversions|ToFloat(Integer) (Math|Float|Round (|(((((((StatBS*2)+IV)*CL)/100)+CL)+5)*MP) (.SPAttack (Utilities|Struct|BreakFPoggermonBaseStats (.BaseStatInformation (Utilities|Struct|BreakFPoggermonBasicInformation _returnvalue)))) (.SPAttack (Utilities|Struct|BreakFPoggermonIV (.PoggerIV (Utilities|Struct|BreakFPoggermonPartyInfo (Variables|Default|GetEncounterPoggermon))))) (Utilities|Struct|BreakFPoggermonPartyInfo (Variables|Default|GetEncounterPoggermon)) (.Value (Utilities|Map|Find (.Stats (Utilities|Struct|BreakFNatures _returnvalue_2)) "SP Attack"))))) (Math|Conversions|ToFloat(Integer) (Math|Float|Round (|(((((((StatBS*2)+IV)*CL)/100)+CL)+5)*MP) (.SPDefense (Utilities|Struct|BreakFPoggermonBaseStats (.BaseStatInformation (Utilities|Struct|BreakFPoggermonBasicInformation _returnvalue)))) (.SPDefense (Utilities|Struct|BreakFPoggermonIV (.PoggerIV (Utilities|Struct|BreakFPoggermonPartyInfo (Variables|Default|GetEncounterPoggermon))))) (Utilities|Struct|BreakFPoggermonPartyInfo (Variables|Default|GetEncounterPoggermon)) (.Value (Utilities|Map|Find (.Stats (Utilities|Struct|BreakFNatures _returnvalue_2)) "SP Defense"))))) (Math|Conversions|ToFloat(Integer) (Math|Float|Round (|(((((((StatBS*2)+IV)*CL)/100)+CL)+5)*MP) (.SPDefense (Utilities|Struct|BreakFPoggermonBaseStats (.BaseStatInformation (Utilities|Struct|BreakFPoggermonBasicInformation _returnvalue)))) (.SPDefense (Utilities|Struct|BreakFPoggermonIV (.PoggerIV (Utilities|Struct|BreakFPoggermonPartyInfo (Variables|Default|GetEncounterPoggermon))))) (Utilities|Struct|BreakFPoggermonPartyInfo (Variables|Default|GetEncounterPoggermon)) (.Value (Utilities|Map|Find (.Stats (Utilities|Struct|BreakFNatures _returnvalue_2)) "SP Defense"))))) (Math|Conversions|ToFloat(Integer) (Math|Float|Round (|(((((((StatBS*2)+IV)*CL)/100)+CL)+5)*MP) (.Speed (Utilities|Struct|BreakFPoggermonBaseStats (.BaseStatInformation (Utilities|Struct|BreakFPoggermonBasicInformation _returnvalue)))) (.Speed (Utilities|Struct|BreakFPoggermonIV (.PoggerIV (Utilities|Struct|BreakFPoggermonPartyInfo (Variables|Default|GetEncounterPoggermon))))) (Utilities|Struct|BreakFPoggermonPartyInfo (Variables|Default|GetEncounterPoggermon)) (.Value (Utilities|Map|Find (.Stats (Utilities|Struct|BreakFNatures _returnvalue_2)) "Speed"))))) (Math|Conversions|ToFloat(Integer) (Math|Float|Round (|(((((((StatBS*2)+IV)*CL)/100)+CL)+5)*MP) (.Speed (Utilities|Struct|BreakFPoggermonBaseStats (.BaseStatInformation (Utilities|Struct|BreakFPoggermonBasicInformation _returnvalue)))) (.Speed (Utilities|Struct|BreakFPoggermonIV (.PoggerIV (Utilities|Struct|BreakFPoggermonPartyInfo (Variables|Default|GetEncounterPoggermon))))) (Utilities|Struct|BreakFPoggermonPartyInfo (Variables|Default|GetEncounterPoggermon)) (.Value (Utilities|Map|Find (.Stats (Utilities|Struct|BreakFNatures _returnvalue_2)) "Speed"))))) (.Accuracy (Utilities|Struct|BreakFPoggermonBaseStats (.BaseStatInformation (Utilities|Struct|BreakFPoggermonBasicInformation _returnvalue)))) (.Accuracy (Utilities|Struct|BreakFPoggermonBaseStats (.BaseStatInformation (Utilities|Struct|BreakFPoggermonBasicInformation _returnvalue)))) (.Evasiveness (Utilities|Struct|BreakFPoggermonBaseStats (.BaseStatInformation (Utilities|Struct|BreakFPoggermonBasicInformation _returnvalue)))) (.Evasiveness (Utilities|Struct|BreakFPoggermonBaseStats (.BaseStatInformation (Utilities|Struct|BreakFPoggermonBasicInformation _returnvalue)))))))
          (Variables|Default|SetEncounterPoggermon _structout))
        (:RowNotFound
          (Development|PrintString "Failed EncounterBp"))))))

(fn RollMoveSlots
  (bind _possiblemoves (Variables|Default|GetPossibleMoves))
  (bind _returnvalue (Utilities|Array|LastIndex _possiblemoves))
  (bind _outrownames (DataTable|GetDataTableRowNames "/Game/CreatureInfo/PoggermonMoveDT.PoggermonMoveDT"))
  (for _array_element _outrownames
    (if (.ReturnValue (Utilities|Map|Find (Utilities|Struct|BreakFPoggermonBaseStats (.PoggerBaseStats (Utilities|Struct|BreakFPoggermonPartyInfo (Variables|Default|GetEncounterPoggermon)))) _array_element))
      (if (<= (.Value (Utilities|Map|Find (Utilities|Struct|BreakFPoggermonBaseStats (.PoggerBaseStats (Utilities|Struct|BreakFPoggermonPartyInfo (Variables|Default|GetEncounterPoggermon)))) _array_element)) (.CurrentLevel (Utilities|Struct|BreakFPoggermonPartyInfo (Variables|Default|GetEncounterPoggermon))))
        (Utilities|Array|Add (Variables|Default|GetPossibleMoves) (.Value (Utilities|Map|Find (Utilities|Struct|BreakFPoggermonBaseStats (.PoggerBaseStats (Utilities|Struct|BreakFPoggermonPartyInfo (Variables|Default|GetEncounterPoggermon)))) _array_element))))))
  (bind _keys (Utilities|Map|Keys (Utilities|Struct|BreakFPoggermonBaseStats (.PoggerBaseStats (Utilities|Struct|BreakFPoggermonPartyInfo (Variables|Default|GetEncounterPoggermon))))))
  (for _index (range 0 3)
    (if (> (Utilities|Array|Length _possiblemoves) 0)
      (bind _returnvalue_2 (Utilities|GetDataTableRow "/Game/CreatureInfo/PoggermonMoveDT.PoggermonMoveDT" (Utilities|Array|Get(acopy) _keys _returnvalue))
        (:then
          (Utilities|Array|AddUnique (Variables|Default|GetMove) (.MoveName (Utilities|Struct|BreakFMoveStruct _returnvalue_2)))
          (Utilities|Array|RemoveIndex (Variables|Default|GetPossibleMoves) _returnvalue)))))
  (bind _structout (Utilities|Struct|SetmembersinFPoggermonPartyInfo (Variables|Default|GetEncounterPoggermon) (Variables|Default|GetMove)))
  (Variables|Default|SetEncounterPoggermon _structout)
  (return))

(fn FindNature
  (switch int (Math|Random|RandomIntegerinRange 0 6)
    (:0
      (Variables|Default|SetNatures "Docile"))
    (:1
      (Variables|Default|SetNatures "Timid"))
    (:2
      (Variables|Default|SetNatures "Lonely"))
    (:3
      (Variables|Default|SetNatures "Adamant"))
    (:4
      (Variables|Default|SetNatures "Modest"))
    (:5
      (Variables|Default|SetNatures "Hasty"))
    (:6
      (Variables|Default|SetNatures "Gentle")))
  (bind _structout (Utilities|Struct|SetmembersinFPoggermonPartyInfo (Variables|Default|GetEncounterPoggermon) (Variables|Default|GetNatures)))
  (Variables|Default|SetEncounterPoggermon _structout))