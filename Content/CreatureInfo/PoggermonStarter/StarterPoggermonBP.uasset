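; Starter Poggermon pickup that a VR player can inspect while their trainer party is still empty.
; Box overlap with the VRPawn caches the pawn, enables input and rolls shininess and gender once into the starter's party info at a fixed starting level; leaving disables input.
; Left index-curl input scans the party for any named Poggermon and, if none exists, calls the pawn's ShowPoggermonDetails with the starter and its Poggerball.
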(event `Roll for Info`
  ; Set Information
  (`/Engine/EditorBlueprintResources/StandardMacros.DoOnce` false
    (:`Completed`
      (if (== (`KismetMathLibrary.RandomIntegerInRange` 1 4096) 1)
        (set `self.is Shiny` true)
        (else
          (set `self.is Shiny` false)))
      (if (>= (`KismetMathLibrary.RandomInteger` 100) 51)
        (set `self.Gender` "NewEnumerator1")
        (else
          (set `self.Gender` "NewEnumerator2")))
      (bind _structout (setmembers `/Game/CreatureInfo/FPoggermonPartyInfo` :`StructRef` (`self.StarterPoggermon`) :`Current Level` 5 :`Gender` (`self.Gender`) :`Is Shiny?` (`self.is Shiny`)))
      (set `self.StarterPoggermon` _structout))))

(event `self.Box.OnComponentBeginOverlap`
  (params (OverlappedComponent :type "PrimitiveComponent Object Reference") (OtherActor :type "Actor Object Reference") (OtherComp :type "PrimitiveComponent Object Reference") (OtherBodyIndex :type Integer) (bFromSweep :type Boolean) (SweepResult :type "HitResult Structure (by ref)"))
  ; SetOverlap
  (`KismetSystemLibrary.PrintString` (`KismetTextLibrary.Conv_TextToString` (`|FormatText` "Overlap: {Actor}" OtherActor)))
  (bind _asvrpawn (cast `/Game/VRTemplate/Blueprints/VRPawn` OtherActor))
  (set `self.Quikish Ref` _asvrpawn)
  (`self.EnableInput` (`GameplayStatics.GetPlayerController` 0))
  (`self.Roll for Info`))

(event `self.Box.OnComponentEndOverlap`
  (params (OverlappedComponent :type "PrimitiveComponent Object Reference") (OtherActor :type "Actor Object Reference") (OtherComp :type "PrimitiveComponent Object Reference") (OtherBodyIndex :type Integer))
  ; SetOverlap
  (cast `/Game/VRTemplate/Blueprints/VRPawn` OtherActor)
  (`self.DisableInput` (`GameplayStatics.GetPlayerController` 0)))

(event `Key|E`
  (params (Key :type "Key Structure"))
  ; Interact With Starter
)

(event `EnhancedInput|/Game/VRTemplate/Input/Actions/Hands/IA_Hand_IndexCurl_Left`
  (params (ActionValue :type "Float (double-precision)") (ElapsedSeconds :type "Float (double-precision)") (TriggeredSeconds :type "Float (double-precision)") (InputAction :type "InputAction Object Reference" :default "/Game/VRTemplate/Input/Actions/Hands/IA_Hand_IndexCurl_Left.IA_Hand_IndexCurl_Left"))
  ; Interact With Starter
  (:`Started`
    (for _array_element (`.TrainerParty_4_2D73034040B613D8451F96B64207EDDF` (break `/Game/ThirdPerson/Blueprints/FTrainerPoggermon` (`/Game/VRTemplate/Blueprints/VRPawn.Trainer Poggermon` (`self.Quikish Ref`))))
      (if (not (== (`.PoggermonName_11_C5D621984448D1224532A0BCA2E58EE2` (break `/Game/CreatureInfo/FPoggermonPartyInfo` _array_element)) "None"))
        (set `self.HasPokemon?` true)
        (break)))
    (if (not (`self.HasPokemon?`))
      (set `PlayerController.bShowMouseCursor` false (`GameplayStatics.GetPlayerController` 0))
      (`/Game/VRTemplate/Blueprints/VRPawn.ShowPoggermonDetails` (`self.Quikish Ref`) (`self.PoggermonName`) (`self.StarterPoggermon`) (`self.Poggerball`)))))

(fn `UserConstructionScript`)